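; BP_Puzzle is an actor that assembles a puzzle from two child-actor item pads and a child-actor gate.
; On BeginPlay it takes the first Objective-interface component from each pad and adds both to its Puzzle component as objectives.
; It then hands the gate's PuzzleGate component to that same Puzzle component, leaving completion logic outside this Blueprint.
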(event EventBeginPlay
  (bind _objectives (Variables|Default|GetObjectives))
  ;[0.15 0.15 0.15 0.5] Set Puzzle Objectives
  (bind _objective (CallFunction|GetObjectivefromItemPad (Variables|Default|GetItemPad)))
  (Utilities|Array|Add (Variables|Default|GetObjectives) _objective)
  (bind _objective_2 (CallFunction|GetObjectivefromItemPad (Variables|Default|GetItemPad2)))
  (Utilities|Array|Add _objectives _objective_2)
  (Class|Puzzle|AddObjectives (Variables|Default|GetPuzzle) _objectives)
  ;[0.15 0.15 0.15 0.5] Set Puzzle Gate
  (bind _asbp_puzzle_gate (Utilities|Casting|CastToBP_PuzzleGate (Variables|/Script/Engine.ChildActorComponent|GetChildActor (Variables|Default|GetPuzzleGate))))
  (Class|Puzzle|SetPuzzleGate (Variables|Default|GetPuzzle) (Actor|GetComponentbyClass _asbp_puzzle_gate "/Script/TalosRecords.PuzzleGate")))

(fn ConstructionScript)

(fn GetObjectivefromItemPad
  (params (ChildActorComponent :type Child%20Actor%20Component%20Object%20Reference))
  (bind _asbp_item_pad (Utilities|Casting|CastToBP_ItemPad (Variables|/Script/Engine.ChildActorComponent|GetChildActor ChildActorComponent)))
  (bind _asobjective (Utilities|Casting|CastToObjective (Utilities|Array|Get(acopy) (Class|Actor|GetComponentsbyInterface _asbp_item_pad "/Script/TalosRecords.Objective"))))
  (return _asobjective))