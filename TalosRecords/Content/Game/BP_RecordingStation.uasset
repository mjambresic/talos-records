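; BP_RecordingStation is an interactable station that drives the player's recording UI and camera effect.
; It caches the player pawn on BeginPlay and responds to the RecordingStation's OnInteract event by adding or removing the player's recording widget and toggling the camera recording effect.
; While recording, Tick pushes the RecordingStation's formatted accumulated time to that widget.
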(event OnInteract(RecordingStation)
  (params (bRecording :type Boolean))
  ;[0.15 0.15 0.15 0.5] Resolve User Interface on Interact
  (if bRecording
    (UserInterface|Viewport|AddtoViewport (Variables|/Game/Game/BP_Player.BP_Player_C|GetWB_Recording (Variables|Default|GetPlayer)) 0)
    (Default|SetCameraRecordingEffectEnabled (Variables|Default|GetPlayer) true)
    (CallFunction|UpdateWidgetCurrentTime)
    (else
      (Widget|RemovefromParent (Variables|/Game/Game/BP_Player.BP_Player_C|GetWB_Recording (Variables|Default|GetPlayer)))
      (Default|SetCameraRecordingEffectEnabled (Variables|Default|GetPlayer) false))))

(event EventTick
  (params (DeltaSeconds :type Float%20%28single-precision%29))
  ;[0.15 0.15 0.15 0.5] Tick
  (CallFunction|UpdateWidgetCurrentTime))

(event EventBeginPlay
  ;[0.15 0.15 0.15 0.5] Initialization
  (bind _asbp_player (Utilities|Casting|CastToBP_Player (Pawn|GetControlledPawn (Game|GetPlayerController 0))))
  (Variables|Default|SetPlayer _asbp_player))

(fn ConstructionScript)

(fn UpdateWidgetCurrentTime
  (bind _recordingstation (Variables|Default|GetRecordingStation))
  (if (Class|RecordingStation|GetIsRecording _recordingstation)
    (Default|SetCurrentTime (Variables|/Game/Game/BP_Player.BP_Player_C|GetWB_Recording (Variables|Default|GetPlayer)) (Class|RecordingStation|GetFormattedAccumulatedTime _recordingstation))))